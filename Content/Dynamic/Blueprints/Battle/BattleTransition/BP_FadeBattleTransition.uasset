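; Battle transition Blueprint that plays a fade to black through a UI widget, then a camera fade.
; StartTransition moves its SceneCaptureComponent2D to the player camera and captures the scene, then shows BP_FadeTransitionUI.
; After a short delay it removes the widget, starts a camera fade from full alpha and immediately signals the transition has ended.
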(event EventStartTransition
  ;[1 1 1] Fade to black
  (Transformation|SetWorldTransform (Variables|Default|GetSceneCaptureComponent2D) (Transformation|GetActorTransform (Variables|/Script/Engine.PlayerController|GetPlayerCameraManager (Game|GetPlayerController 0))) false false)
  (Rendering|SceneCapture|CaptureScene (Variables|Default|GetSceneCaptureComponent2D) :!class /Script/Engine.SceneCaptureComponent2D)
  (bind _returnvalue (UserInterface|CreateWidget "/Game/Dynamic/Blueprints/UI/BP_FadeTransitionUI.BP_FadeTransitionUI_C"))
  (UserInterface|Viewport|AddtoViewport _returnvalue 0)
  (Utilities|FlowControl|Delay 0.5)
  (Widget|RemovefromParent _returnvalue)
  (CameraFades|StartCameraFade :self (Variables|/Script/Engine.PlayerController|GetPlayerCameraManager (Game|GetPlayerController 0)) :FromAlpha 1.0 :Duration 0.5 :bHoldWhenFinished true)
  (Default|CallOnTransitionEnded))

(fn ConstructionScript
  (|CallParentFunction))