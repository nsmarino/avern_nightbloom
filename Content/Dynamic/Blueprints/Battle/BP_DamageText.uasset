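; Actor that shows a floating damage, heal or MP number for a target unit in battle.
; On BeginPlay it gets the BP_DamageTextUI from its widget component and passes it the amount, unit and heal/MP flags.
; It binds to the end of the Bounce animation, then destroys itself when that finishes.
; The finish handler unbinds from the Appear animation rather than Bounce.
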(event Custom|OnAnimationFinishedHandler
  ;[1 1 1] Show damage
  (Class|UserWidget|UnbindAllfromAnimationFinished (Variables|Default|GetdamageTextUI) (Variables|/Game/Dynamic/Blueprints/UI/BP_DamageTextUI.BP_DamageTextUI_C|GetAppear (Variables|Default|GetdamageTextUI)))
  (Actor|DestroyActor))

(event EventBeginPlay
  ;[1 1 1] Show damage
  (bind _output_get (Variables|Default|SetdamageTextUI (.AsBP%20Damage%20Text%20UI (Utilities|Casting|CastToBP_DamageTextUI (UserInterface|GetUserWidgetObject (Variables|Default|GetDamageTextUIWidget))))))
  (Class|UserWidget|BindtoAnimationFinished _output_get (Variables|/Game/Dynamic/Blueprints/UI/BP_DamageTextUI.BP_DamageTextUI_C|GetBounce _output_get) (delegate Custom|OnAnimationFinishedHandler))
  (Default|SetDamage (Variables|Default|GetdamageTextUI) (Variables|Default|Getdamage) (Variables|Default|GettargetUnit) (Variables|Default|GetisHeal) (Variables|Default|GetisMP)))

(fn ConstructionScript)