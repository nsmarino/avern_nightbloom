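; Double Hit skill for unit battles that attacks the current target twice, with each hit driven by an animation notify.
; The attacker optionally moves to the target through the BattleController before the skill animation plays.
; Each notify damages the target if it is still alive and applies buffs when damage is dealt.
; When the animation ends, the unit moves back if needed, then signals that the skill is used.
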(event Custom|OnUnitMovedBackHandler
  ;[1 1 1] Attack twice
  (Default|CallOnSkillUsed))

(event Custom|OnUnitMovedToTargetHandler
  ;[1 1 1] Move to target
  (CallFunction|PlaySkillAnimation))

(event EventUseSkillonNotify
  (bind _battlecontroller (Variables|Default|GetbattleController))
  ;[1 1 1] Attack twice
  (bind _isunitdead (Default|IsUnitDead (Variables|/Game/Dynamic/Blueprints/Battle/BP_BattleController.BP_BattleController_C|GetcurrentTargetUnit _battlecontroller)))
  (if (not _isunitdead)
    (bind _ishit (Default|DealDamage _battlecontroller 0 1.0))
    (if _ishit
      (CallFunction|ApplyBuffs (Utilities|Array|MakeArray (Variables|/Game/Dynamic/Blueprints/Battle/BP_BattleController.BP_BattleController_C|GetcurrentTargetUnit (Variables|Default|GetbattleController)))))))

(event EventUseSkill
  ;[1 1 1] Move to target
  (if (Variables|/Game/Dynamic/Blueprints/Battle/BP_BattleController.BP_BattleController_C|GetshouldUnitsMoveToTarget (Variables|Default|GetbattleController))
    (Default|MovetoTarget (Variables|Default|GetbattleController) (Transformation|GetWorldLocation (Variables|/Game/Dynamic/Blueprints/Units/BP_UnitBase.BP_UnitBase_C|GetAttackerLocation (Variables|/Game/Dynamic/Blueprints/Battle/BP_BattleController.BP_BattleController_C|GetcurrentTargetUnit (Variables|Default|GetbattleController)))) (delegate Custom|OnUnitMovedToTargetHandler) true)
    (else
      (CallFunction|PlaySkillAnimation))))

(event EventOnSkillAnimationEnded
  ;[1 1 1] Attack twice
  (if (Variables|/Game/Dynamic/Blueprints/Battle/BP_BattleController.BP_BattleController_C|GetshouldUnitsMoveToTarget (Variables|Default|GetbattleController))
    (Default|MovetoTarget (Variables|Default|GetbattleController) (Variables|/Game/Dynamic/Blueprints/Units/BP_UnitBase.BP_UnitBase_C|GetinitialLocation (Variables|/Game/Dynamic/Blueprints/Battle/BP_BattleController.BP_BattleController_C|GetcurrentAttackingUnit (Variables|Default|GetbattleController))) (delegate Custom|OnUnitMovedBackHandler) false)
    (else
      (Default|CallOnSkillUsed))))

(fn ConstructionScript
  (|CallParentFunction))